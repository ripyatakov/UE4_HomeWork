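; Game mode for a chunk-based runner that builds the track and holds game speed, coin count, game-over and bonus state.
; BeginPlay lays GenerationRange random chunks along X; SpawnChunk rolls chances for coins, walls, moving walls and bonuses at chunk markers, with obstacles only rolled after a coin spawns.
; SlowAll and UntouchableAll apply timed bonuses, halving speed or setting invulnerability.
; Death kills the player character once.
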(event `SlowAll`
  (`GameplayStatics.SpawnSound2D` "/Game/Sounds/bonusSlow.bonusSlow" 0.3 1.0 0.0 null)
  (if (`self.Slowable`)
    (set `self.Game Speed` (* (`self.Game Speed`) 2.0)))
  (set `self.Game Speed` (/ (`self.Game Speed`) 2.0))
  (set `self.Slowable` true)
  (`KismetSystemLibrary.Delay` (`self.BonusDuration`))
  (set `self.Game Speed` (* (`self.Game Speed`) 2.0))
  (set `self.Slowable` false))

(event `self.ReceiveBeginPlay`
  (`self.GameStart`))

(event `UntouchableAll`
  (`GameplayStatics.SpawnSound2D` "/Game/Sounds/bonusUntouchable.bonusUntouchable" 0.1 1.0 0.0 null)
  (set `self.UnTouchable` true)
  (`KismetSystemLibrary.Delay` (`self.BonusDuration`))
  (set `self.UnTouchable` false))

(fn `CoinCollected`
  (set `self.CoinsCollected` (+ (`self.CoinsCollected`) 1))
  (`GameplayStatics.SpawnSound2D` "/Game/Sounds/coin.coin" 0.1 1.0 0.0 null))

(fn `Death`
  (if (not (`self.IsGameOver`))
    (bind _asthird_person_character (cast `/Game/ThirdPersonBP/Blueprints/ThirdPersonCharacter` (`GameplayStatics.GetPlayerCharacter` 0)))
    (`/Game/ThirdPersonBP/Blueprints/ThirdPersonCharacter.Dead` _asthird_person_character)
    (set `self.IsGameOver` true)))

(fn `SpawnBonus`
  (params (Pos :type "Vector Structure"))
  (bind _returnvalue (`KismetMathLibrary.MakeTransform` Pos (struct :`Pitch` 90.0)))
  (if (<= (`KismetMathLibrary.RandomFloat`) 0.5)
    (`|SpawnActorFromClass` (`self.BonusUntouchable`) _returnvalue "Undefined" "OverrideRootScale" null null)
    (else
      (`|SpawnActorFromClass` (`self.BonusSlow`) _returnvalue "Undefined" "OverrideRootScale" null null))))

(fn `SpawnChunk`
  (bind _chunksarr (`self.ChunksArr`))
  (bind _returnvalue (`KismetMathLibrary.RandomInteger` (`KismetArrayLibrary.Array_Length` _chunksarr)))
  (bind _output_get (set `self.Last_Chunk_Pos` (+ (`self.Last_Chunk_Pos`) (* (4000.0 0.0 0.0) 1))))
  (bind _returnvalue_2 (`|SpawnActorFromClass` (`|GetArrayItem` _chunksarr _returnvalue) (`KismetMathLibrary.MakeTransform` _output_get) "Undefined" "OverrideRootScale" null null))
  (if (< (`KismetMathLibrary.RandomFloat`) (`self.SpawnCoinChance`))
    (bind _coinspositions (`/Game/ChunksBP/BP_Chunk_Parent.CoinsPositions` _returnvalue_2))
    (`self.SpawnCoin` (`SceneComponent.K2_GetComponentLocation` (`|GetArrayItem` _coinspositions (`KismetMathLibrary.RandomInteger` (`KismetArrayLibrary.Array_Length` _coinspositions)))))
    (if (< (`KismetMathLibrary.RandomFloat`) (`self.SpawnWallChance`))
      (bind _wallspositions (`/Game/ChunksBP/BP_Chunk_Parent.WallsPositions` _returnvalue_2))
      (`self.SpawnWall` (`SceneComponent.K2_GetComponentLocation` (`|GetArrayItem` _wallspositions (`KismetMathLibrary.RandomInteger` (`KismetArrayLibrary.Array_Length` _wallspositions)))))
      (elif (and (== _returnvalue 1) (< (`KismetMathLibrary.RandomFloat`) (`self.SpawnMovingWallChance`)))
        (bind _movingwallspositions (`/Game/ChunksBP/BP_Chunk_Parent.MovingWallsPositions` _returnvalue_2))
        (`self.SpawnMovingWall` (`SceneComponent.K2_GetComponentLocation` (`|GetArrayItem` _movingwallspositions (`KismetMathLibrary.RandomInteger` (`KismetArrayLibrary.Array_Length` _movingwallspositions))))))))
  (if (< (`KismetMathLibrary.RandomFloat`) (`self.SpawnBonusChance`))
    (bind _bonuspositions (`/Game/ChunksBP/BP_Chunk_Parent.BonusPositions` _returnvalue_2))
    (`self.SpawnBonus` (`SceneComponent.K2_GetComponentLocation` (`|GetArrayItem` _bonuspositions (`KismetMathLibrary.RandomInteger` (`KismetArrayLibrary.Array_Length` _bonuspositions)))))))

(fn `SpawnCoin`
  (params (Pos :type "Vector Structure"))
  (`|SpawnActorFromClass` (`self.Coin`) (`KismetMathLibrary.MakeTransform` Pos (struct :`Pitch` 90.0)) "Undefined" "OverrideRootScale" null null))

(fn `SpawnMovingWall`
  (params (Pos :type "Vector Structure"))
  (`|SpawnActorFromClass` (`self.MovingWall`) (`KismetMathLibrary.MakeTransform` Pos (struct :`Pitch` 90.0)) "Undefined" "OverrideRootScale" null null))

(fn `SpawnWall`
  (params (Pos :type "Vector Structure"))
  (`|SpawnActorFromClass` (`self.Wall`) (`KismetMathLibrary.MakeTransform` Pos (struct :`Pitch` 90.0)) "Undefined" "OverrideRootScale" null null))

(fn `UserConstructionScript`)