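; BP_Chunk_Parent is the base level chunk for a game that spawns its track chunk by chunk.
; On BeginPlay it gathers its placement points for coins, walls, moving walls and bonuses into separate position arrays.
; When a ThirdPersonCharacter overlaps ChunkSpawnTrigger, it tells BP_Game_Mode to spawn another chunk.
; SpawnStarted is an empty function here, and nothing in this Blueprint uses the gathered arrays.
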(event `self.ReceiveBeginPlay`
  (bind _coinspositions (`self.CoinsPositions`))
  (bind _wallspositions (`self.WallsPositions`))
  (bind _movingwallspositions (`self.MovingWallsPositions`))
  (bind _bonuspositions (`self.BonusPositions`))
  (bind _coinspositions_2 (`self.CoinsPositions`))
  (`KismetArrayLibrary.Array_Add` _coinspositions_2 (`self.CoinP1`))
  (`KismetArrayLibrary.Array_Add` _coinspositions_2 (`self.CoinP2`))
  (`KismetArrayLibrary.Array_Add` _coinspositions_2 (`self.CoinP3`))
  (`KismetArrayLibrary.Array_Add` _coinspositions_2 (`self.CoinP4`))
  (`KismetArrayLibrary.Array_Add` _coinspositions (`self.CoinP5`))
  (`KismetArrayLibrary.Array_Add` _coinspositions (`self.CoinP6`))
  (`KismetArrayLibrary.Array_Add` _coinspositions (`self.CoinP7`))
  (`KismetArrayLibrary.Array_Add` _coinspositions (`self.CoinP8`))
  (`KismetArrayLibrary.Array_Add` _wallspositions (`self.WallP1`))
  (`KismetArrayLibrary.Array_Add` _wallspositions (`self.WallP2`))
  (`KismetArrayLibrary.Array_Add` _movingwallspositions (`self.MovingWallP1`))
  (`KismetArrayLibrary.Array_Add` _movingwallspositions (`self.MovingWallP2`))
  (`KismetArrayLibrary.Array_Add` _bonuspositions (`self.BonusP1`))
  (`KismetArrayLibrary.Array_Add` _bonuspositions (`self.BonusP2`)))

(event `self.ChunkSpawnTrigger.OnComponentBeginOverlap`
  (params (OverlappedComponent :type "PrimitiveComponent Object Reference") (OtherActor :type "Actor Object Reference") (OtherComp :type "PrimitiveComponent Object Reference") (OtherBodyIndex :type Integer) (bFromSweep :type Boolean) (SweepResult :type "HitResult Structure (by ref)"))
  (cast `/Game/ThirdPersonBP/Blueprints/ThirdPersonCharacter` OtherActor)
  (bind _asbp_game_mode (cast `/Game/GameMode/BP_Game_Mode` (`GameplayStatics.GetGameMode`)))
  (`/Game/GameMode/BP_Game_Mode.SpawnChunk` _asbp_game_mode))

(fn `UserConstructionScript`)