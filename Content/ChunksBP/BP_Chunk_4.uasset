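; BP_Chunk_4 is a chunk Blueprint with a rotating fan and two kill volumes for the player.
; Each tick it runs the parent tick, then rolls BigFanLol at a rate scaled by the game mode's GameSpeed.
; When a ThirdPersonCharacter begins overlapping Box or Box1, both handlers share one path that calls Death on BP_Game_Mode.
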(event `self.ReceiveTick`
  (params (DeltaSeconds :type "Float (single-precision)"))
  (`parent.ReceiveTick` DeltaSeconds)
  (bind _asbp_game_mode (cast `/Game/GameMode/BP_Game_Mode` (`GameplayStatics.GetGameMode`)))
  (`SceneComponent.K2_AddLocalRotation` (`self.Big Fan lol`) (`KismetMathLibrary.MakeRotator` (* DeltaSeconds (* (`/Game/GameMode/BP_Game_Mode.Game Speed` _asbp_game_mode) 30.0))) false false))

(event `self.Box.OnComponentBeginOverlap`
  (params (OverlappedComponent :type "PrimitiveComponent Object Reference") (OtherActor :type "Actor Object Reference") (OtherComp :type "PrimitiveComponent Object Reference") (OtherBodyIndex :type Integer) (bFromSweep :type Boolean) (SweepResult :type "HitResult Structure (by ref)"))
  (cast `/Game/ThirdPersonBP/Blueprints/ThirdPersonCharacter` OtherActor)
  (bind _asbp_game_mode (cast `/Game/GameMode/BP_Game_Mode` (`GameplayStatics.GetGameMode`) :!label _label))
  (`/Game/GameMode/BP_Game_Mode.Death` _asbp_game_mode))

(event `self.Box1.OnComponentBeginOverlap`
  (params (OverlappedComponent :type "PrimitiveComponent Object Reference") (OtherActor :type "Actor Object Reference") (OtherComp :type "PrimitiveComponent Object Reference") (OtherBodyIndex :type Integer) (bFromSweep :type Boolean) (SweepResult :type "HitResult Structure (by ref)"))
  (cast `/Game/ThirdPersonBP/Blueprints/ThirdPersonCharacter` OtherActor)
  (goto _label))

(fn `UserConstructionScript`
  (`parent.UserConstructionScript`))