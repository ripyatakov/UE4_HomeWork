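; Coin pickup actor that spins in the level and is collected when the player touches it.
; Tick rotates the Cylinder2 component around its roll axis at a constant, frame-rate-independent speed.
; The Box overlap checks the overlapping component for the Player tag, notifies BP_Game_Mode through CoinCollected, then destroys the coin.
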(event `self.ReceiveTick`
  (params (DeltaSeconds :type "Float (single-precision)"))
  (`SceneComponent.K2_AddLocalRotation` (`self.Cylinder2`) (`KismetMathLibrary.MakeRotator` (* DeltaSeconds 90.0)) false false))

(event `self.Box.OnComponentBeginOverlap`
  (params (OverlappedComponent :type "PrimitiveComponent Object Reference") (OtherActor :type "Actor Object Reference") (OtherComp :type "PrimitiveComponent Object Reference") (OtherBodyIndex :type Integer) (bFromSweep :type Boolean) (SweepResult :type "HitResult Structure (by ref)"))
  (if (`ActorComponent.ComponentHasTag` OtherComp "Player")
    (bind _asbp_game_mode (cast `/Game/GameMode/BP_Game_Mode` (`GameplayStatics.GetGameMode`)))
    (`/Game/GameMode/BP_Game_Mode.CoinCollected` _asbp_game_mode)
    (`self.K2_DestroyActor`)))

(fn `UserConstructionScript`)