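; Wall obstacle actor that kills the player on contact unless the game mode's UnTouchable state is active.
; Each Tick polls BP_Game_Mode and switches the Cube between solid collision with the basic wall material and no collision with a glass material.
; A Box overlap with a component tagged Player calls Death on the game mode when UnTouchable is off.
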(event `self.ReceiveTick`
  (params (DeltaSeconds :type "Float (single-precision)"))
  (bind _cube (`self.Cube`))
  (bind _cube_2 (`self.Cube`))
  (bind _asbp_game_mode (cast `/Game/GameMode/BP_Game_Mode` (`GameplayStatics.GetGameMode`)))
  (if (`/Game/GameMode/BP_Game_Mode.UnTouchable` _asbp_game_mode)
    (`PrimitiveComponent.SetCollisionEnabled` _cube_2 "NoCollision")
    (`PrimitiveComponent.SetMaterial` _cube_2 0 "/Game/StarterContent/Materials/M_Glass.M_Glass")
    (else
      (`PrimitiveComponent.SetCollisionEnabled` _cube "QueryAndPhysics")
      (`PrimitiveComponent.SetMaterial` _cube 0 "/Game/StarterContent/Materials/M_Basic_Wall.M_Basic_Wall"))))

(event `self.Box.OnComponentBeginOverlap`
  (params (OverlappedComponent :type "PrimitiveComponent Object Reference") (OtherActor :type "Actor Object Reference") (OtherComp :type "PrimitiveComponent Object Reference") (OtherBodyIndex :type Integer) (bFromSweep :type Boolean) (SweepResult :type "HitResult Structure (by ref)"))
  (bind _asbp_game_mode (cast `/Game/GameMode/BP_Game_Mode` (`GameplayStatics.GetGameMode`)))
  (if (and (`ActorComponent.ComponentHasTag` OtherComp "Player") (not (`/Game/GameMode/BP_Game_Mode.UnTouchable` _asbp_game_mode)))
    (`/Game/GameMode/BP_Game_Mode.Death` _asbp_game_mode)))

(fn `UserConstructionScript`)