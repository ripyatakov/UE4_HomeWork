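; FanWall_BP is a fan wall actor that spins continuously during play.
; Each Tick it casts the game mode to BP_Game_Mode and adds local roll rotation scaled by frame time and that mode's GameSpeed, so the spin follows game speed.
; Without that game mode it stays still, and the construction script only calls its parent.
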(event `self.ReceiveTick`
  (params (DeltaSeconds :type "Float (single-precision)"))
  (`parent.ReceiveTick` DeltaSeconds)
  (bind _asbp_game_mode (cast `/Game/GameMode/BP_Game_Mode` (`GameplayStatics.GetGameMode`)))
  (`self.K2_AddActorLocalRotation` (`KismetMathLibrary.MakeRotator` (* (`/Game/GameMode/BP_Game_Mode.Game Speed` _asbp_game_mode) (* DeltaSeconds 40.0)))))

(fn `UserConstructionScript`
  (`parent.UserConstructionScript`))